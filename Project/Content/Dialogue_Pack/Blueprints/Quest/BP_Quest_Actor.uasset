(event Custom|EventUpdate
  (params (QuestName :type Name) (RewardEXP :type Integer) (FinishQuestNow :type Boolean) (UpdateObjective :type Name))
  (bind (_exist _finished_ _currentprogress) (CallFunction|FuncUpdateQuest QuestName RewardEXP FinishQuestNow UpdateObjective)) ; please dont call func's from outside. otherwise dispatchers will not work\nthis is the base update logic
  (if _exist
    ;[1 0.5946 0.2964] dispatchers, to fire events
    (Default|CallDispUpdate QuestName _finished_ _currentprogress)
    (else
      (Development|PrintString "QUEST DOES NOT EXIST!"))))

(event Custom|CloseJournal
  (bind _widget (Variables|NonEditable|GetWidget))
  ;[1 0.6491 0.162] this is to close from(dialogue_component)
  ;[1 1 1] closes the widget but not the mouse and focus
  (Default|ClearObjectives _widget) ; clear objective selection on close
  (Widget|RemovefromParent _widget)
  (Input|SetIgnoreLookInput (Game|GetPlayerController 0) false)
  (Variables|NonEditable|SetJournal? false))

(event Custom|EventCreate
  (params (QuestName :type Name) (QuestLength :type Integer) (FirstObjective :type Name))
  (CallFunction|FuncCreateQuest QuestName QuestLength FirstObjective) ; please dont call func's from outside. otherwise dispatchers will not work\nthis is the base create logic
  ;[1 0.5946 0.2964] dispatchers, to fire events
  (Default|CallDispCreate QuestName))

(event EventBeginPlay
  ;[0.4695 0.6162 1] get widget reference
  (bind _returnvalue (UserInterface|CreateWidget "/Game/Dialogue_Pack/Blueprints/Quest/HUD/Quest_HUD.Quest_HUD_C"))
  (Variables|NonEditable|SetWidget _returnvalue)
  (bind _returnvalue_2 (UserInterface|CreateWidget "/Game/Dialogue_Pack/Blueprints/Quest/HUD/Quest_Reminder.Quest_Reminder_C"))
  (bind _output_get (Variables|NonEditable|SetReminder_Widget _returnvalue_2))
  (UserInterface|Viewport|AddtoViewport _output_get 0))

(event Input|KeyboardEvents|J
  (params (Key :type Key%20Structure :default "AnyKey"))
  (bind _returnvalue (Game|GetPlayerController 0))
  (bind _widget (Variables|NonEditable|GetWidget))
  ;[0.3538 1 0.7763] open/close journal logic on J button(quest actor always receive player input)
  (:Pressed
    (if (not (Variables|NonEditable|GetDialogue?))
      (if (Variables|NonEditable|GetJournal?)
        (Default|ClearObjectives _widget) ; clear objective selection on close
        (Widget|RemovefromParent _widget)
        (Variables|/Script/Engine.PlayerController|SetbShowMouseCursor _returnvalue false)
        (Input|SetIgnoreLookInput _returnvalue false)
        (Input|SetInputModeGameOnly _returnvalue)
        (Variables|NonEditable|SetJournal? false)
        (else
          (UserInterface|Viewport|AddtoViewport _widget 0)
          (Variables|/Script/Engine.PlayerController|SetbShowMouseCursor _returnvalue true)
          (Input|SetIgnoreLookInput _returnvalue true)
          (Input|SetInputModeGameandUI _returnvalue (Variables|NonEditable|GetWidget) "DoNotLock" false)
          (Variables|NonEditable|SetJournal? true))))))

(fn ConstructionScript)

(fn FuncUpdateQuest
  (params (QuestName :type Name) (RewardEXP :type Integer) (FinishQuestNow :type Boolean) (UpdateObjective :type Name))
  (bind _questprogresslength (Variables|NonEditable|GetQuestProgressLength))
  (bind _currentobjective (Variables|NonEditable|GetCurrentObjective))
  (bind _currentindex (Variables|NonEditable|GetCurrentIndex))
  (bind _currentindex_2 (Variables|NonEditable|GetCurrentIndex))
  (bind _currentindex_3 (Variables|NonEditable|GetCurrentIndex))
  (bind _questcurrentprogress (Variables|NonEditable|GetQuestCurrentProgress))
  (bind _questcurrentprogress_2 (Variables|NonEditable|GetQuestCurrentProgress))
  (bind _item (Utilities|Array|Get(acopy) _questcurrentprogress _currentindex_2))
  (bind _item_2 (Utilities|Array|Get(acopy) _questprogresslength _currentindex))
  (bind _item_3 (Utilities|Array|Get(acopy) _questcurrentprogress_2 _currentindex))
  (CallFunction|FuncSetVariables (Utilities|Array|FindItem (Variables|NonEditable|GetQuestArray) QuestName) QuestName FinishQuestNow UpdateObjective)
  ;[1 0.5166 0.2203] check if quest exists or finished
  (bind _exist (CallFunction|FuncCheckQuest (Variables|NonEditable|GetCurrentName)))
  (bind _output_get (Variables|NonEditable|SetCurrentExist _exist)) ; set for easy sorting
  (if _output_get
    ;[0.4608 1 0.3476] check if quest needs to be finished right now
    (if (Variables|NonEditable|GetCurrentFinish)
      ;[0.2664 1 0.1888] update journal widget
      (Default|UpdateWidget (Variables|NonEditable|GetWidget) (Variables|NonEditable|GetCurrentIndex) (Variables|NonEditable|GetCurrentObjective) :!label _label)
      (Default|CompleteWidget (Variables|NonEditable|GetWidget) _currentindex_3)
      ;[0.2664 1 0.1888] sets a completed quest array
      (Utilities|Array|SetArrayElem (Variables|NonEditable|GetCompletedArray) _currentindex_3 true true)
      ;[1 0.7987 0.396] update floating reminder
      (Default|QuestUpdated (Variables|NonEditable|GetReminder_Widget) true (Utilities|Text|ToText(Name) (Variables|NonEditable|GetCurrentName)))
      ;[0.3 1 1] sets exist/finished/progress on output
      (return (Variables|NonEditable|GetCurrentExist) true _item)
      (else
        ;[0.654 0.439 1] set objective length and name to array
        (Utilities|Array|SetArrayElem (Variables|NonEditable|GetQuestCurrentProgress) (Variables|NonEditable|GetCurrentIndex) (+ _item_3 1) true)
        (Utilities|Array|SetArrayElem (Variables|NonEditable|GetObjectiveArray) (Variables|NonEditable|GetCurrentIndex) (Variables|NonEditable|GetCurrentObjective) true)
        (if (or (== _item_3 _item_2) (== _item_2 0)) ; if true = completed\nif false = updated
          (goto _label)
          (else
            ;[1 0.7165 0.2914] on quest updated, update journal widget and floating reminder
            (Default|UpdateWidget (Variables|NonEditable|GetWidget) (Variables|NonEditable|GetCurrentIndex) _currentobjective)
            (Default|QuestUpdated (Variables|NonEditable|GetReminder_Widget) false (Utilities|Text|ToText(Name) _currentobjective)))))))
  (return (Variables|NonEditable|GetCurrentExist) false _item))

(fn FuncCheckQuest
  (params (QuestName :type Name))
  (bind _questarray (Variables|NonEditable|GetQuestArray))
  (bind _completedarray (Variables|NonEditable|GetCompletedArray))
  (bind _returnvalue (Utilities|Array|FindItem _questarray QuestName))
  ;[1 1 1] makes a quick check of quest if its exist/not completed or otherwise
  (if (Utilities|Array|IsValidIndex _completedarray _returnvalue)
    (return (and (Utilities|Array|ContainsItem _questarray QuestName) (not (Utilities|Array|Get(acopy) _completedarray _returnvalue)))) ; otherwise check if it exist and not completed
    (else
      (return false) ; if completed index is false, then quest probably never created
    )))

(fn FuncCreateQuest
  (params (QuestName :type Name) (QuestLength :type Integer) (FirstObjective :type Name))
  (bind _questarray (Variables|NonEditable|GetQuestArray))
  (bind _returnvalue (Utilities|Array|LastIndex _questarray))
  ;[1 0.124 0.1638] if same quest exist then do nothing
  (if (not (Utilities|Array|ContainsItem (Variables|NonEditable|GetQuestArray) QuestName))
    ;[0.4371 0.5215 1] sets quest name into array
    (Utilities|Array|SetArrayElem _questarray (Utilities|Array|Length _questarray) QuestName true)
    ;[0.3749 1 0.7544] set quest length to array
    (Utilities|Array|SetArrayElem (Variables|NonEditable|GetQuestProgressLength) _returnvalue QuestLength true)
    ;[0.32 0.9402 1] set current progress to 0
    ; (at creation)
    (Utilities|Array|SetArrayElem (Variables|NonEditable|GetQuestCurrentProgress) _returnvalue (Class|KismetSystemLibrary|MakeLiteralInteger) true)
    ;[0.2575 0.5776 1] set objective to array
    (Utilities|Array|SetArrayElem (Variables|NonEditable|GetObjectiveArray) _returnvalue FirstObjective true)
    ;[0.426 0.2344 1] set false to completed array
    (Utilities|Array|SetArrayElem (Variables|NonEditable|GetCompletedArray) _returnvalue (Class|KismetSystemLibrary|MakeLiteralBool false) true)
    ;[1 0.7553 0.2464] set values to widget
    (Default|AddWidget (Variables|NonEditable|GetWidget) QuestName FirstObjective _returnvalue)
    ;[1 0.8254 0.3297] spawn floating reminder
    (Default|QuestReceived (Variables|NonEditable|GetReminder_Widget) (Utilities|Text|ToText(Name) QuestName))))

(fn FuncSetVariables
  (params (CurrentIndex :type Integer) (CurrentName :type Name) (CurrentFinish :type Boolean) (CurrentObjective :type Name))
  ;[1 1 1] saves the current variables to easy access inside blueprints
  ; (each variable of currently updated quest)
  (Variables|NonEditable|SetCurrentName CurrentName)
  (Variables|NonEditable|SetCurrentObjective CurrentObjective)
  (Variables|NonEditable|SetCurrentIndex CurrentIndex)
  (Variables|NonEditable|SetCurrentFinish CurrentFinish))