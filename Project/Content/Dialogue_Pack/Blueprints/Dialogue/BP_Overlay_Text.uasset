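; Floating 3D text actor for the dialogue system, showing either the owner's name or timed overlay replies above the speaking character.
; Each update pulls the reply through DialogueHUD, attaches to that speaker, plays animation and sound, then waits the calculated delay; random mode stops after one line.
; Ending fires quest and choice events, optionally switches dialogue state, then destroys itself; pausing saves the reply index.
; Tick billboards the widget, clamping camera pitch to avoid flipping.
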(event Custom|Start_Overlay
  (params (Dialogue_Component :type BP%20Dialogue%20Component%20Object%20Reference) (Dialogue_HUD :type Dialogue%20HUD%20Object%20Reference) (Name? :type Boolean) (Unpaused? :type Boolean))
  ;[0.4018 0.6503 1] Start overlay and set dialogue component, event, and update overlay
  (Variables|Default|SetDialogue_Component Dialogue_Component)
  (Variables|NonEditable|SetDialogue_HUD Dialogue_HUD)
  (if Name?
    (CallFunction|SetWidget "Visible" "Visible" Name?)
    (else
      (CallFunction|UpdateOverlay Unpaused?)))
  (CallFunction|AttachTransform Name?))

(event Custom|End_Overlay
  (bind _dialogue_component (Variables|Default|GetDialogue_Component))
  (bind _dialogue_component_2 (Variables|Default|GetDialogue_Component))
  ;[0.2563 1 0.145] on overlay update events, reset, and destroy overlay actor
  (Utilities|FlowControl|Sequence ; first fire events then stop dialogue
    (:then_0
      (Default|UpdateQuest _dialogue_component 2) ; update quest before overlay end
      (Utilities|IsValid _dialogue_component ; check if quest is not destroyed this actor
        (:Is%20Valid
          (Default|ChoiceEvent _dialogue_component 2) ; set choice event for overlays
        )
        (:Is%20Not%20Valid
          (Actor|DestroyActor :!label _label) ; destroy overlay on end
        )))
    (:then_1
      (Utilities|IsValid (Variables|Default|GetDialogue_Component) ; if actor was not destroyed by choice
        (:Is%20Valid
          (if (Variables|NonEditable|GetChangeState?) ; get if we need to change state by overlay
            (Variables|/Game/Dialogue_Pack/Blueprints/Dialogue/BP_Dialogue_Component.BP_Dialogue_Component_C|SetCurrent_State _dialogue_component_2 (Variables|NonEditable|GetLinkedState)) ; set state if bool is true
          )
          (Default|StopTalking _dialogue_component_2) ; stop dialogue to reset variables
          (goto _label))
        (:Is%20Not%20Valid
          (goto _label))))))

(event Custom|Update_Overlay
  (params (Unpause? :type Boolean))
  (bind _dialogue_hud (Variables|NonEditable|GetDialogue_HUD))
  ;[0.447 0.9701 1] update checks validness if true update text, if false end overlay sequence
  (if Unpause?
    (Variables|/Game/Dialogue_Pack/Blueprints/Dialogue/HUD/Dialogue_HUD.Dialogue_HUD_C|SetReplyState (Variables|NonEditable|GetDialogue_HUD) (Variables|/Game/Dialogue_Pack/Blueprints/Dialogue/BP_Dialogue_Component.BP_Dialogue_Component_C|GetPaused_State (Variables|Default|GetDialogue_Component))) ; set reply state to paused if unpaused
  )
  (CallFunction|SetVariables) ; set overlay variables first
  (bind _update_ (Default|UpdateReplyState (Variables|NonEditable|GetDialogue_HUD) 2))
  (if _update_
    (Default|InterruptDelay (Variables|NonEditable|GetDialogue_HUD)) ; set interrupting delay
    (CallFunction|AttachTransform false) ; update attach
    (Default|PlayAnimSound (Variables|NonEditable|GetDialogue_HUD) 2) ; play anim and sound for reply character
    ;[0.447 0.9701 1] sets widget, and calculates delay to second reply, if exist or end it if random
    (CallFunction|SetWidget "Visible" "Visible" false) ; sets widget to visible, and set text from reply
    (Default|CalculateDelay _dialogue_hud) ; calculate delay of text or audio
    (Utilities|FlowControl|RetriggerableDelay (Variables|/Game/Dialogue_Pack/Blueprints/Dialogue/HUD/Dialogue_HUD.Dialogue_HUD_C|GetText_Delay _dialogue_hud))
    (if (Variables|NonEditable|GetRandom?) ; if random is true, end at first phrase
      (CallFunction|EndOverlay) ; finish it
      (else
        (CallFunction|UpdateOverlay false) ; update to next reply
      ))
    (else
      (CallFunction|EndOverlay) ; finish it, if there is no more replies
    )))

(event Custom|End_Paused
  ;[0.2563 1 0.145] on overlay update events, reset, and destroy overlay actor
  (Variables|/Game/Dialogue_Pack/Blueprints/Dialogue/BP_Dialogue_Component.BP_Dialogue_Component_C|SetPaused_State (Variables|Default|GetDialogue_Component) (- (Variables|/Game/Dialogue_Pack/Blueprints/Dialogue/HUD/Dialogue_HUD.Dialogue_HUD_C|GetReplyState (Variables|NonEditable|GetDialogue_HUD)) 1))
  (Default|StopTalking (Variables|Default|GetDialogue_Component)) ; stop dialogue to reset variables
  (Actor|DestroyActor) ; destroy overlay on end
)

(event EventTick
  (params (DeltaSeconds :type Float%20%28single-precision%29))
  (bind _returnvalue (Game|GetPlayerCameraManager 0))
  (bind _returnvalue_2 (Camera|GetCameraRotation _returnvalue))
  (bind (_roll _pitch _yaw) (Math|Rotator|BreakRotator _returnvalue_2))
  ;[1 0.7445 0.2598] set text to face camera each tick
  (Variables|/Script/Engine.PlayerCameraManager|SetViewPitchMin _returnvalue -89.0) ; those to prevent text glitchy flipping\nbecause 90 pitch conflict with 360 yaw\n(you can set it anywhere)
  (Variables|/Script/Engine.PlayerCameraManager|SetViewPitchMax _returnvalue 89.0) ; those to prevent text glitchy flipping\nbecause 90 pitch conflict with 360 yaw\n(you can set it anywhere)
  (Transformation|SetWorldRotation (Variables|Default|Get3DWidget) (Math|Rotator|MakeRotator _roll (* _pitch -1.0) (- _yaw 1.8e+02)) false false) ; simply inverse camera rotation to text's and set it
)

(fn ConstructionScript
  ;[1 1 1] set scale to absolute, to prevent it from scaling
  (Variables|/Script/Engine.SceneComponent|SetbAbsoluteScale (Variables|Default|Get3DWidget) true))

(fn SetVariables
  (bind _dialogue_component (Variables|Default|GetDialogue_Component))
  (bind _dialogue_tree (Variables|/Game/Dialogue_Pack/Blueprints/Dialogue/BP_Dialogue_Component.BP_Dialogue_Component_C|GetDialogue_Tree _dialogue_component))
  (bind _current_state (Variables|/Game/Dialogue_Pack/Blueprints/Dialogue/BP_Dialogue_Component.BP_Dialogue_Component_C|GetCurrent_State _dialogue_component))
  (bind _item (Utilities|Array|Get(acopy) _dialogue_tree _current_state))
  (bind _overlay (Utilities|Struct|BreakTree_Struct _item))
  (bind (_overlay_replies _overlay_settings _quest _random_ _changestate_ _linktostate) (Utilities|Struct|BreakOverlay_Struct _overlay))
  ;[1 1 1] gets variables and store it inside widget
  (Variables|NonEditable|SetRandom? _random_)
  (Variables|NonEditable|SetChangeState? _changestate_)
  (Variables|NonEditable|SetLinkedState _linktostate)
  (if (Variables|NonEditable|GetRandom?)
    ;[1 1 1] if random is true then randomly set reply state from array(so npc will say one random reply from array)
    (Variables|/Game/Dialogue_Pack/Blueprints/Dialogue/HUD/Dialogue_HUD.Dialogue_HUD_C|SetReplyState (Variables|NonEditable|GetDialogue_HUD) (Math|Random|RandomIntegerinRange 0 (Utilities|Array|LastIndex _overlay_replies))) ; set reply state to dialogue_HUD
  ))

(fn AttachTransform
  (params (Name? :type Boolean))
  (bind _dialogue_hud (Variables|NonEditable|GetDialogue_HUD))
  (bind _dialogue_component (Variables|Default|GetDialogue_Component))
  (bind _dialogue_component_2 (Variables|Default|GetDialogue_Component))
  (bind _dialogue_component_3 (Variables|Default|GetDialogue_Component))
  (bind _returnvalue (Components|GetOwner _dialogue_component_2))
  (bind _characterindex (Variables|/Game/Dialogue_Pack/Blueprints/Dialogue/HUD/Dialogue_HUD.Dialogue_HUD_C|GetCharacterIndex _dialogue_hud))
  (bind _characters_list (Variables|/Game/Dialogue_Pack/Blueprints/Dialogue/BP_Dialogue_Component.BP_Dialogue_Component_C|GetCharacters_List _dialogue_component_3))
  (bind _item (Utilities|Array|Get(acopy) _characters_list _characterindex))
  (bind _returnvalue_2 (Transformation|GetActorTransform _returnvalue))
  (bind _returnvalue_3 (Transformation|GetActorTransform _item))
  (bind (_location _rotation _scale) (Math|Transform|BreakTransform _returnvalue_2))
  (bind (_location_2 _rotation_2 _scale_2) (Math|Transform|BreakTransform _returnvalue_3))
  ;[1 1 1] sets currently talking player's transform and attaches to that actor(to show floating overlay text)
  (if Name?
    (Transformation|SetWorldTransform (Variables|Default|GetDefaultSceneRoot) (Math|Transform|MakeTransform (+ _location (Math|Vector|MakeVector 0.0 0.0 (.Text_Height (Utilities|Struct|BreakNPC_Settings_Struct (Variables|/Game/Dialogue_Pack/Blueprints/Dialogue/BP_Dialogue_Component.BP_Dialogue_Component_C|GetNPC_Settings (Variables|Default|GetDialogue_Component)))))) _rotation _scale) false false)
    (Transformation|AttachActorToActor _returnvalue "None" "KeepWorld" "KeepWorld" "KeepWorld" true)
    (else
      (Transformation|SetWorldTransform (Variables|Default|GetDefaultSceneRoot) (Math|Transform|MakeTransform (+ _location_2 (Math|Vector|MakeVector 0.0 0.0 (Math|Float|SelectFloat (.Cam_Height (Utilities|Struct|BreakPlayer_Settings_Struct (Variables|/Game/Dialogue_Pack/Blueprints/Dialogue/BP_Dialogue_Component.BP_Dialogue_Component_C|GetPlayer_Settings _dialogue_component))) (Utilities|Array|Get(acopy) (.Text_Height (Utilities|Struct|BreakNPC_Additional_Settings_Struct (Variables|/Game/Dialogue_Pack/Blueprints/Dialogue/BP_Dialogue_Component.BP_Dialogue_Component_C|GetCharacters_Settings _dialogue_component))) (Variables|/Game/Dialogue_Pack/Blueprints/Dialogue/HUD/Dialogue_HUD.Dialogue_HUD_C|GetCharacterIndex (Variables|NonEditable|GetDialogue_HUD))) (== (Utilities|Array|LastIndex (Variables|/Game/Dialogue_Pack/Blueprints/Dialogue/BP_Dialogue_Component.BP_Dialogue_Component_C|GetCharacters_List (Variables|Default|GetDialogue_Component))) (Variables|/Game/Dialogue_Pack/Blueprints/Dialogue/HUD/Dialogue_HUD.Dialogue_HUD_C|GetCharacterIndex (Variables|NonEditable|GetDialogue_HUD)))))) _rotation_2 _scale_2) false false)
      (Transformation|AttachActorToActor _item "None" "KeepWorld" "KeepWorld" "KeepWorld" true))))

(fn SetWidget
  (params (HiddenBox :type ESlateVisibility%20Enum) (HiddenOverlay :type ESlateVisibility%20Enum) (Name? :type Boolean))
  ;[1 1 1] hide/show and set text of widget
  (bind _asdialogue_overlay (Utilities|Casting|CastToDialogue_Overlay (UserInterface|GetUserWidgetObject (Variables|Default|Get3DWidget)))
    (:then
      (if Name?
        ;[1 1 1] sets floating name widget and color
        (Variables|/Game/Dialogue_Pack/Blueprints/Dialogue/HUD/Dialogue_Overlay.Dialogue_Overlay_C|SetOverlay_Text _asdialogue_overlay (Utilities|Text|ToText(String) (Variables|/Game/Dialogue_Pack/Blueprints/Dialogue/BP_Dialogue_Component.BP_Dialogue_Component_C|GetOwnerName (Variables|Default|GetDialogue_Component))))
        (Appearance|SetColorandOpacity _asdialogue_overlay "(R=1.000000,G=0.675418,B=0.000000,A=1.000000)" :!class /Script/UMG.UserWidget)
        (else
          (Widget|SetVisibility _asdialogue_overlay (select (.Hide_Floating_Overlay? (Utilities|Struct|BreakDialogue_Settings_Struct (Variables|/Game/Dialogue_Pack/Blueprints/Dialogue/BP_Dialogue_Component.BP_Dialogue_Component_C|GetDialogue_Settings (Variables|Default|GetDialogue_Component)))) "Hidden" HiddenOverlay))
          (Widget|SetVisibility (Variables|/Game/Dialogue_Pack/Blueprints/Dialogue/HUD/Dialogue_HUD.Dialogue_HUD_C|GetDialogue_Overlay_Box (Variables|NonEditable|GetDialogue_HUD)) HiddenBox)
          (Variables|/Game/Dialogue_Pack/Blueprints/Dialogue/HUD/Dialogue_Overlay.Dialogue_Overlay_C|SetOverlay_Text _asdialogue_overlay (Variables|/Game/Dialogue_Pack/Blueprints/Dialogue/HUD/Dialogue_HUD.Dialogue_HUD_C|GetAnswerText (Variables|NonEditable|GetDialogue_HUD))))))
    (:CastFailed
      (Development|PrintString "Cast to overlay widget failed")
      (CallFunction|EndOverlay))))