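; Dialogue camera rig that switches between the player/choice camera and several angled shots of the speaking actor.
; Each switch deactivates all cameras first; auto mode randomly loops left, right and medium shots.
; Manual mode indexes a construction-built array mirroring Enum_CameraList, falling back to the last valid camera on None unless auto is enabled, and sets ValidCam for the dialogue HUD.
; Optional placeholder actor meshes are destroyed at construction or BeginPlay.
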(event Custom|DeactivateCams
  ;[1 0 0] deactivates all cameras before setting active one
  ; "necessary, add any new created camera here also"
  (Components|Activation|SetActive (Variables|Default|GetC_R) false false))

(event Custom|Auto_Cam
  ;[1 0.7707 0.1674] sets random reply (auto cams), (facing Actor at different angles)
  (CallFunction|DeactivateCams)
  (Utilities|FlowControl|MultiGate true true -1 ; loop and random switch cameras (left/right/med)
    (:Out%200
      (Components|Activation|SetActive (Variables|Default|GetC_R) true false))
    (:Out%201
      (Components|Activation|SetActive (Variables|Default|GetC_L) true false))
    (:Out%202
      (Components|Activation|SetActive (Variables|Default|GetC_M) true false))))

(event Custom|CreateCameraList
  ;[0.3241 0.3008 1] calls by construct
  (Variables|Default|SetCameraArray (Utilities|Array|MakeArray 0 (Variables|Default|GetC_L) (Variables|Default|GetC_R) (Variables|Default|GetC_M) (Variables|Default|GetC_T) (Variables|Default|GetC_TB) 0 0 0 0 0)) ; the array index list is equal to enum index list for manual scenic camera's
)

(event Custom|DialogueCam
  ;[0.2825 0.8394 1] set basic player dialogue cam active, also choice camera
  (CallFunction|DeactivateCams)
  (Components|Activation|SetActive (Variables|Default|GetPlayer_Dialogue_Cam) true false))

(event Custom|Manual_Cam
  (params (Index :type Integer) (AutoEnabled? :type Boolean))
  (bind _cameraarray (Variables|Default|GetCameraArray))
  (bind _item (Utilities|Array|Get(acopy) _cameraarray Index))
  ;[0.2661 1 0.3223] sets manual cams from struct array
  (CallFunction|DeactivateCams)
  (Utilities|IsValid _item ; index (0) is always invalid because its None from enum_CameraList\nso latest valid camera will remain active at None
    (:Is%20Valid
      (Components|Activation|SetActive _item true false)
      (Variables|Default|SetLastValidCam _item) ; latest valid cam
      (Variables|NonEditable|SetValidCam true :!label _label) ; sets that cam is valid so switch will happen
    )
    (:Is%20Not%20Valid
      (if AutoEnabled? ; if auto is enabled, dont set last valid cam to active
        _
        (else
          (Utilities|IsValid (Variables|Default|GetLastValidCam) ; gets if last valid cam is valid
            (:Is%20Valid
              (Components|Activation|SetActive (Variables|Default|GetLastValidCam) true false) ; this activates at "None"
              (goto _label))
            (:Is%20Not%20Valid
              _))))
      (Variables|NonEditable|SetValidCam false) ; sets that there is absolutely no valid cam, so in dialogue_HUD will be no camera switch \n(can happen if first camera from array is None)
    )))

(event EventBeginPlay
  ;[0.3583 0.3382 1] if you forgot to hide mesh, it will auto destroy on beginplay
  (if (Variables|Default|GetShowMesh?)
    (Components|DestroyComponent (Variables|Default|GetActor))))

(fn ConstructionScript
  ;[1 1 1] show optional mesh and create camera list
  (if (Variables|Default|GetShowMesh?)
    _
    (else
      (Components|DestroyComponent (Variables|Default|GetActor))))
  (CallFunction|CreateCameraList))