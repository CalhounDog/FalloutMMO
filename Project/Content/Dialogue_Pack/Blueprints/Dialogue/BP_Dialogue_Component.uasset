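; Actor component that runs an NPC's branching conversations with the player from a state-indexed DialogueTree.
; StartDialogue allows one active conversation, validates the state, then locks input, positions both actors, and spawns per-character cameras and the HUD.
; Greetings, choices and floating overlay lines can trigger events, animation, sound and BP_Quest_Actor updates.
; Tick handles proximity name tags and distance-based overlay pausing, while StopTalking restores input, camera and any temporary state.
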(event Custom|StartDialogue
  ;[0.005281 1 0] Start Dialogue
  (bind _active_dialogue_ (UpdateState|CheckDialogue)) ; check if player is in dialogue if false then start dialogue
  (if _active_dialogue_
    ;[1 0.7062 0.1914] dispatch event for dialogue starting
    (Default|CallDispStarted false)
    (else
      (Default|CallDispStarted true)
      (Variables|NonEditable|SetInDialogue? true) ; dialogue start bool
      ;[0.239 1 0.1314] Start Dialogue Sequence
      (UpdateDialogue|SetDialogue))))

(event Custom|SetEvents
  ;[0.287 0.8597 1] set basic events, if dialogue can be started
  ; (check dialogue setfunc)
  ;[0.7054 0.779 1] Block player movement on dialogue
  (UpdatePlayer|IgnoreMovement true)
  ;[1 0.8754 0.7284] fix rotation and location and set player cam to dialogue
  (UpdatePlayer|SweepActors)
  (UpdatePlayer|SpawnDialogueCams)
  ;[0.6446 0.552 1] spawn dialogue cams BP
  ; (must be before widget and after loc fix)
  (UpdatePlayer|SetPlayerCam false)
  ;[0.4766 1 0.5863] spawn widget and add to viewport
  (UpdateDialogue|SpawnWidget false))

(event Custom|ChoiceEvent
  (params (Type? :type Integer))
  (bind _current_state (Variables|NonEditable|GetCurrent_State))
  (bind _dialogue_tree (Variables|Dialogue|GetDialogue_Tree))
  (bind _chosen_index (Variables|NonEditable|GetChosen_Index))
  (bind _item (Utilities|Array|Get(acopy) _dialogue_tree _current_state))
  (bind (_greetings _choice _overlay) (Utilities|Struct|BreakTree_Struct _item))
  (bind (_overlay_replies _overlay_settings _quest _random_ _changestate_ _linktostate _overlayevent _deactivate) (Utilities|Struct|BreakOverlay_Struct _overlay))
  (bind (_greetings_replies _greetings_settings _quest_2 _exit_ _exittostate _greetevent _deactivate_2) (Utilities|Struct|BreakGreetings_Struct _greetings))
  (bind _item_2 (Utilities|Array|Get(acopy) _choice _chosen_index))
  (bind (_choice_text _choice_replies _choice_settings _quest_3 _linktostate_2 _exit__2 _choiceevent _deactivate_3) (Utilities|Struct|BreakChoice_Struct _item_2))
  ;[0.116 0.3229 1] sets choice event,
  ; example if you have (non quest related choice), and you need to update some npc's dialogue values
  (if (Utilities|Select :Index Type? :Option%200 _greetevent :Option%201 _choiceevent :Option%202 _overlayevent)
    (Default|CallDispChoice))
  (Variables|NonEditable|SetDeactive? (Utilities|Select :Index Type? :Option%200 _deactivate_2 :Option%201 _deactivate_3 :Option%202 _deactivate)))

(event Custom|UpdateQuest
  (params (Type? :type Integer))
  (bind _current_state (Variables|NonEditable|GetCurrent_State))
  (bind _chosen_index (Variables|NonEditable|GetChosen_Index))
  (bind _dialogue_tree (Variables|Dialogue|GetDialogue_Tree))
  (bind _item (Utilities|Array|Get(acopy) _dialogue_tree _current_state))
  (bind (_greetings _choice _overlay) (Utilities|Struct|BreakTree_Struct _item))
  (bind _quest (Utilities|Struct|BreakGreetings_Struct _greetings))
  (bind _quest_2 (Utilities|Struct|BreakOverlay_Struct _overlay))
  (bind _item_2 (Utilities|Array|Get(acopy) _choice _chosen_index))
  (bind _quest_3 (Utilities|Struct|BreakChoice_Struct _item_2))
  (bind _returnvalue (Utilities|Select :Index Type? :Option%200 _quest :Option%201 _quest_3 :Option%202 _quest_2))
  (bind (_questname _questobjective _objectivelength_ _create_) (Utilities|Struct|BreakQuest_Struct _returnvalue))
  ;[0.4791 0.3001 1] sets quest event, create/update or finish within the dialogue
  (if (Utilities|Name|NotEqual(Name) _questname "None") ; quest named none will be ignored
    (if _create_ ; create or update?
      (Default|EventCreate (Variables|NonEditable|GetQuest_Actor) _questname _objectivelength_ _questobjective)
      (else
        (Default|EventUpdate (Variables|NonEditable|GetQuest_Actor) _questname 0 false _questobjective)))))

(event Custom|StopTalking
  (bind _dialogue_overlay (Variables|NonEditable|GetDialogue_Overlay))
  (bind _dialogue_hud (Variables|NonEditable|GetDialogue_HUD))
  (bind _name_overlay (Variables|NonEditable|GetName_Overlay))
  ;[0 0.6557 1] Dialogue End Sequence
  (Variables|NonEditable|SetInDialogue? false)
  (Variables|/Game/Dialogue_Pack/Blueprints/Quest/BP_Quest_Actor.BP_Quest_Actor_C|SetDialogue? (Variables|NonEditable|GetQuest_Actor) false)
  (UpdatePlayer|IgnoreMovement false)
  (UpdateState|TemporarilyState 0 true) ; reset temporary state
  (UpdatePlayer|SetPlayerCam true) ; reset player camera(and destroy dialogue_cams)
  (Utilities|IsValid _dialogue_hud
    (:Is%20Valid
      (Widget|RemovefromParent _dialogue_hud) ; remove widget if exist
    )
    (:Is%20Not%20Valid
      _))
  ;[1 0.09001 0.04025] destroy all parts of this component(overlays)
  (Utilities|IsValid _name_overlay
    (:Is%20Valid
      (Actor|DestroyActor _name_overlay))
    (:Is%20Not%20Valid
      _))
  (Utilities|IsValid _dialogue_overlay
    (:Is%20Valid
      (Actor|DestroyActor _dialogue_overlay))))

(event EventTick
  (params (DeltaSeconds :type Float%20%28single-precision%29))
  ;[1 0.6033 0.06383] optional tick event show name above NPC head, if player is close
  (UpdateDialogue|ShowOverlayName)
  (UpdateDialogue|PauseOverlay))

(event EventBeginPlay
  ;[1 1 1] gets reference to quest actor
  ; (dont spawn more than one quest actor)
  (bind _outactors (Actor|GetAllActorsOfClass "/Game/Dialogue_Pack/Blueprints/Quest/BP_Quest_Actor.BP_Quest_Actor_C"))
  (Variables|NonEditable|SetQuest_Actor (Utilities|Array|Get(acopy) _outactors))
  ;[1 1 1] store involved actors into array
  (UpdatePlayer|SetActors))

(event EventEndPlay
  (params (EndPlayReason :type EEndPlayReason%20Enum :default "Destroyed"))
  ;[1 0.006772 0] stop talking on being destroyed(to destroy every part of this component)
  (CallFunction|StopTalking))

(fn IgnoreMovement
  (params (On? :type Boolean))
  (bind _returnvalue (Game|GetPlayerController 0))
  (bind _returnvalue_2 (Game|GetPlayerController 0))
  (bind _quest_actor (Variables|NonEditable|GetQuest_Actor))
  ;[1 1 1] just basic logic, show mouse, lock player, and focus widget(or unblock player, hide mouse and unfocus widget
  (Utilities|IsValid (Game|GetPlayerController 0) ; if destroyed
    (:Is%20Valid
      (if On? ; true blocks player(false unblocks)
        (Variables|/Script/Engine.PlayerController|SetbShowMouseCursor _returnvalue true)
        (Input|SetIgnoreLookInput _returnvalue true)
        (Input|SetIgnoreMoveInput _returnvalue true)
        (Input|SetInputModeGameandUI _returnvalue (Variables|NonEditable|GetDialogue_HUD) "DoNotLock" false)
        ;[1 1 1] blocks quest journal while in dialogue
        (Variables|/Game/Dialogue_Pack/Blueprints/Quest/BP_Quest_Actor.BP_Quest_Actor_C|SetDialogue? _quest_actor true)
        (Default|CloseJournal _quest_actor)
        (else
          (Variables|/Script/Engine.PlayerController|SetbShowMouseCursor _returnvalue_2 false)
          (Input|SetIgnoreLookInput _returnvalue_2 false)
          (Input|SetIgnoreMoveInput _returnvalue_2 false)
          (Input|SetInputModeGameOnly _returnvalue_2))))))

(fn UpdateQuestions
  (bind _dialogue_hud (Variables|NonEditable|GetDialogue_HUD))
  (bind _dialogue_hud_2 (Variables|NonEditable|GetDialogue_HUD))
  (bind _dialogue_hud_3 (Variables|NonEditable|GetDialogue_HUD))
  (bind _questionlist (Variables|/Game/Dialogue_Pack/Blueprints/Dialogue/HUD/Dialogue_HUD.Dialogue_HUD_C|GetQuestionList _dialogue_hud))
  ;[1 1 1] Remove and Clear old question list
  (Utilities|IsValid _dialogue_hud
    (:Is%20Valid
      (for _array_element _questionlist
        (Widget|RemovefromParent _array_element))
      (Utilities|Array|Clear _questionlist)
      ;[1 1 1] for each loop add questions(choices)
      (for (_array_element_2 _array_index) (.Choice (Utilities|Struct|BreakTree_Struct (Utilities|Array|Get(acopy) (Variables|Dialogue|GetDialogue_Tree) (Variables|NonEditable|GetCurrent_State))))
        ;[1 1 1] gets choice button's text and adds button(if text is empty dont spawn a button)
        (if (Utilities|Enum|NotEqual(Enum) (.Choice_Text (Utilities|Struct|BreakChoice_Struct _array_element_2)) (Utilities|Text|MakeLiteralText ""))
          ;[1 1 1] create button widget and store references inside
          (bind _returnvalue (UserInterface|CreateWidget "/Game/Dialogue_Pack/Blueprints/Dialogue/HUD/Dialogue_Choice.Dialogue_Choice_C"))
          (Widget|Panel|AddChild (Variables|/Game/Dialogue_Pack/Blueprints/Dialogue/HUD/Dialogue_Choice_Box.Dialogue_Choice_Box_C|GetChoiceBox (Variables|/Game/Dialogue_Pack/Blueprints/Dialogue/HUD/Dialogue_HUD.Dialogue_HUD_C|GetDialogue_Choice_Box (Variables|NonEditable|GetDialogue_HUD))) _returnvalue)
          ;[1 1 1] set necessary variables inside each choice and create questionlist array
          (Variables|/Game/Dialogue_Pack/Blueprints/Dialogue/HUD/Dialogue_Choice.Dialogue_Choice_C|SetChoice_Text _returnvalue (.Choice_Text (Utilities|Struct|BreakChoice_Struct _array_element_2)))
          (bind _output_get (Variables|/Game/Dialogue_Pack/Blueprints/Dialogue/HUD/Dialogue_Choice.Dialogue_Choice_C|SetSelection_Index _returnvalue _array_index))
          (Variables|/Game/Dialogue_Pack/Blueprints/Dialogue/HUD/Dialogue_Choice.Dialogue_Choice_C|SetLinkedState _returnvalue (.LinkToState (Utilities|Struct|BreakChoice_Struct _array_element_2)))
          (Variables|/Game/Dialogue_Pack/Blueprints/Dialogue/HUD/Dialogue_Choice.Dialogue_Choice_C|SetExit? _returnvalue (.Exit? (Utilities|Struct|BreakChoice_Struct _array_element_2)))
          (Variables|/Game/Dialogue_Pack/Blueprints/Dialogue/HUD/Dialogue_Choice.Dialogue_Choice_C|SetDialogueComponent _returnvalue self)
          (Variables|/Game/Dialogue_Pack/Blueprints/Dialogue/HUD/Dialogue_Choice.Dialogue_Choice_C|SetParent_HUD _returnvalue _dialogue_hud_2)
          (Utilities|Array|SetArrayElem (Variables|/Game/Dialogue_Pack/Blueprints/Dialogue/HUD/Dialogue_HUD.Dialogue_HUD_C|GetQuestionList _dialogue_hud_2) _output_get _returnvalue true)))
      ;[1 1 1] check if there is valid choices in this state
      (bind _choiceexist_ (UpdateState|CheckValidness 1))
      (if _choiceexist_
        (UpdateDialogue|SetChosen true) ; update chosen colors(used ones)
        (if (Variables|NonEditable|GetInDialogue?) ; check if player is in dialogue, so dont set camera if questions was updated out of dialogue\nit basicly resets to default dialogue cam when choices appear
          (UpdatePlayer|SetPlayerCam false) ; set player cam to dialogue when choices appear
        )
        ;[1 1 1] set gamepad or keyboard selection color
        (if (Variables|/Game/Dialogue_Pack/Blueprints/Dialogue/HUD/Dialogue_HUD.Dialogue_HUD_C|GetGamePad? _dialogue_hud_3)
          (Default|SetFocusColor _dialogue_hud_3))
        (else
          ;[1 1 1] if there is no choices at this state then stop dialogue to prevent jam
          (CallFunction|StopTalking))))))

(fn SetDialogue
  ;[1 1 1] this happens at dialogue start
  ;[1 1 1] if inactive then go to overlays
  (if (Variables|NonEditable|GetDeactive?)
    ;[1 1 1] checks validity of overlays then starts them or stops dialogue
    (bind _overlayexist_ (UpdateState|CheckValidness 2 :!label _label))
    (if _overlayexist_ ; if no overlays stop dialogue(if true start overlay sequence)
      ;[1 1 1] stop dialogue if there is no valid choices and greetings,
      ; then stop talking and play overlays
      (UpdateDialogue|SpawnWidget true)
      (UpdateDialogue|ShowOverlayDialogue (Variables|NonEditable|GetPaused?))
      (else
        (CallFunction|StopTalking)))
    (else
      ;[1 1 1] check for at least 1 valid greeting or choice at current state to start dialogue
      ; otherwise stop dialogue(or start overlays)
      (bind _greetexist_ (UpdateState|CheckValidness))
      (if _greetexist_
        _
        (else
          (bind _choiceexist_ (UpdateState|CheckValidness 1))
          (if _choiceexist_ ; if there is no valid greet and choices then try to go to overlays
            _
            (else
              (goto _label)))))
      ;[1 1 1] prepare necessary events
      (CallFunction|SetEvents)
      ;[1 1 1] starts greetings sequence inside widget
      (Default|UpdateGreetings (Variables|NonEditable|GetDialogue_HUD)))))

(fn SweepActors
  (if (.Dont_Sweep_NPC? (Utilities|Struct|BreakDialogue_Settings_Struct (Variables|Default|GetDialogue_Settings))) ; if npc must be static and remain at same location without sweep fix
    ;[1 1 1] first fix player position then rotate player to face static NPC
    (UpdatePlayer|SweepPlayer true 1.5e+02) ; try to sweep player until we hit something
    (bind _success (UpdatePlayer|RotatePlayer)) ; if player was behind "static" NPC, then teleport player to face NPC from front
    (if (not _success)
      (UpdatePlayer|SweepPlayer false 1.5e+02) ; teleport player to front of NPC
      (UpdatePlayer|RotatePlayer) ; and rotate again to fix view
    )
    (else
      ;[1 1 1] first rotate player, and npc to face each other, then sweep player and npc
      (UpdatePlayer|RotatePlayer) ; try to rotate player to face npc
      (UpdatePlayer|RotateNPC) ; then rotate npc to face player
      (UpdatePlayer|SweepPlayer true 1.5e+02) ; sweep player until we hit something
      (UpdatePlayer|SweepNPC true 1.5e+02) ; and sweep npc until he hits something
    )))

(fn TemporarilyState
  (params (Set_State :type Integer) (Reset? :type Boolean))
  ;[1 1 1] if you need to temporarily change state, and save older one
  ; (example use, you did crime and npc wants arrest you, after that on dialogue end, state restores to latest one)
  ; (recommended to stop dialogue before changing current state,)
  (if Reset?
    (if (Variables|NonEditable|GetTemporarily_State?)
      (Variables|NonEditable|SetCurrent_State (Variables|NonEditable|GetTemporary_State))
      (Variables|NonEditable|SetTemporarily_State? false))
    (elif (Variables|NonEditable|GetTemporarily_State?)
      _
      (else
        (Variables|NonEditable|SetTemporary_State (Variables|NonEditable|GetCurrent_State))
        (Variables|NonEditable|SetCurrent_State Set_State)
        (Variables|NonEditable|SetTemporarily_State? true)
        (UpdateDialogue|UpdateQuestions))))
  (return))

(fn SetChosen
  (params (Update? :type Boolean))
  (bind _chosenstruct (Variables|NonEditable|GetChosenStruct))
  (bind _current_state (Variables|NonEditable|GetCurrent_State))
  (bind _dialogue_hud (Variables|NonEditable|GetDialogue_HUD))
  (bind _current_state_2 (Variables|NonEditable|GetCurrent_State))
  (bind _dialogue_hud_2 (Variables|NonEditable|GetDialogue_HUD))
  (bind _chosenstruct_2 (Variables|NonEditable|GetChosenStruct))
  (bind _questionlist (Variables|/Game/Dialogue_Pack/Blueprints/Dialogue/HUD/Dialogue_HUD.Dialogue_HUD_C|GetQuestionList _dialogue_hud))
  (bind _questionlist_2 (Variables|/Game/Dialogue_Pack/Blueprints/Dialogue/HUD/Dialogue_HUD.Dialogue_HUD_C|GetQuestionList _dialogue_hud_2))
  ;[1 1 1] check to store or update
  (if (.Chosen_Color? (Utilities|Struct|BreakDialogue_Settings_Struct (Variables|Default|GetDialogue_Settings)))
    (if Update?
      ;[1 1 1] updates chosen replies, and sets their color to gray.
      (if (Utilities|Array|IsValidIndex _chosenstruct_2 _current_state_2)
        (for (_array_element _array_index) (Utilities|Struct|BreakChosen_Struct (Utilities|Array|Get(acopy) _chosenstruct_2 _current_state_2))
          (Utilities|IsValid _array_element
            (:Is%20Valid
              (if (Utilities|Array|IsValidIndex _questionlist_2 _array_index)
                (Appearance|SetColorandOpacity (Utilities|Array|Get(acopy) _questionlist_2 _array_index) (Variables|/Game/Dialogue_Pack/Blueprints/Dialogue/HUD/Dialogue_Choice.Dialogue_Choice_C|GetChosen_Color _array_element) :!class /Script/UMG.UserWidget)))))
        (elif (Utilities|Array|IsValidIndex _questionlist)
          (Utilities|Array|SetArrayElem (Variables|NonEditable|GetChosenStruct) (Variables|NonEditable|GetCurrent_State) (Utilities|Struct|MakeChosen_Struct _questionlist) true)))
      (else
        ;[1 1 1] store chosen replies to array
        (if (Utilities|Array|IsValidIndex _chosenstruct _current_state)
          (Variables|NonEditable|SetChosenArray (Utilities|Struct|BreakChosen_Struct (Utilities|Array|Get(acopy) _chosenstruct _current_state))) ; this array is needed as reference otherwise set array element for struct will not work
          (Variables|/Game/Dialogue_Pack/Blueprints/Dialogue/HUD/Dialogue_Choice.Dialogue_Choice_C|SetChosen_Color (Utilities|Array|Get(acopy) (Variables|NonEditable|GetChosenArray) (Variables|NonEditable|GetChosen_Index)) "(R=0.250000,G=0.250000,B=0.250000,A=1.000000)") ; set your custom used color here
          (Utilities|Array|SetArrayElem (Variables|NonEditable|GetChosenStruct) (Variables|NonEditable|GetCurrent_State) (Utilities|Struct|MakeChosen_Struct (Variables|NonEditable|GetChosenArray)) true))))))

(fn SetPlayerCam
  (params (Reset? :type Boolean))
  (bind _returnvalue (Game|GetPlayerController 0))
  (bind _dialogue_cams (Variables|NonEditable|GetDialogue_Cams))
  (bind _returnvalue_2 (Utilities|Array|LastIndex _dialogue_cams))
  (bind _item (Utilities|Array|Get(acopy) _dialogue_cams _returnvalue_2))
  ;[1 1 1] sets player basic dialogue cam
  (if Reset?
    (Utilities|IsValid _returnvalue ; if destroyed
      (:Is%20Valid
        (Game|Player|SetViewTargetwithBlend _returnvalue (Game|GetPlayerCharacter 0) 0.0 "VTBlend_Linear" 0.0 false)
        ;[1 1 1] destroy dialogue cams, at dialogue end while reseting player's default cam
        (for _array_element (Variables|NonEditable|GetDialogue_Cams)
          (Utilities|IsValid _array_element
            (:Is%20Valid
              (Actor|DestroyActor _array_element))))))
    (else
      (Utilities|IsValid _item
        (:Is%20Valid
          (Default|DialogueCam _item)
          (Game|Player|SetViewTargetwithBlend (Game|GetPlayerController 0) _item 0.0 "VTBlend_Linear" 0.0 false))))))

(fn SpawnDialogueCams
  (bind _characters_list (Variables|NonEditable|GetCharacters_List))
  (bind _characters_settings (Variables|Default|GetCharacters_Settings))
  (bind _cam_height (Utilities|Struct|BreakNPC_Additional_Settings_Struct _characters_settings))
  (bind _returnvalue (Utilities|Array|LastIndex _characters_list))
  ;[1 1 1] this spawns and stores dialogue cams for each character and npc that involved in this dialogue, this is necessary blueprint that holds every dialogue cam inside
  ; it destroys at each dialogue end inside (reset_player_cams) func
  (for (_array_element _array_index) (Variables|NonEditable|GetCharacters_List)
    (Utilities|IsValid _array_element
      (:Is%20Valid
        (bind _returnvalue_2 (Game|SpawnActorfromClass "/Game/Dialogue_Pack/Blueprints/Dialogue/BP_Dialogue_Cams.BP_Dialogue_Cams_C" (Transformation|GetActorTransform _array_element) "AlwaysSpawn" 0 0))
        (Utilities|Array|SetArrayElem (Variables|NonEditable|GetDialogue_Cams) _array_index _returnvalue_2 true)
        (Transformation|AttachActorToActor _returnvalue_2 _array_element "None" "SnapToTarget" "SnapToTarget" "SnapToTarget" false) ; attach to npc (if he will move)\n(snap to target to fix transform)
        ;[1 1 1] set height of additional npc's from array
        (if (Utilities|Array|IsValidIndex _cam_height _array_index)
          (Transformation|SetRelativeLocation (Variables|/Game/Dialogue_Pack/Blueprints/Dialogue/BP_Dialogue_Cams.BP_Dialogue_Cams_C|GetHeight_Offset (Utilities|Array|Get(acopy) (Variables|NonEditable|GetDialogue_Cams) _array_index)) (Math|Vector|MakeVector 0.0 0.0 (Utilities|Array|Get(acopy) _cam_height _array_index)) false false)))))
  ;[1 1 1] set cam height of NPC and Player's by index
  (Transformation|SetRelativeLocation (Variables|/Game/Dialogue_Pack/Blueprints/Dialogue/BP_Dialogue_Cams.BP_Dialogue_Cams_C|GetHeight_Offset (Utilities|Array|Get(acopy) (Variables|NonEditable|GetDialogue_Cams) (- _returnvalue 1))) (Math|Vector|MakeVector 0.0 0.0 (.Cam_Height (Utilities|Struct|BreakNPC_Settings_Struct (Variables|Default|GetNPC_Settings)))) false false)
  (Transformation|SetRelativeLocation (Variables|/Game/Dialogue_Pack/Blueprints/Dialogue/BP_Dialogue_Cams.BP_Dialogue_Cams_C|GetHeight_Offset (Utilities|Array|Get(acopy) (Variables|NonEditable|GetDialogue_Cams) _returnvalue)) (Math|Vector|MakeVector 0.0 0.0 (.Cam_Height (Utilities|Struct|BreakPlayer_Settings_Struct (Variables|Default|GetPlayer_Settings)))) false false))

(fn CheckValidness
  (params (Type? :type Integer))
  (bind _current_state (Variables|NonEditable|GetCurrent_State))
  (bind _dialogue_tree (Variables|Dialogue|GetDialogue_Tree))
  (bind _item (Utilities|Array|Get(acopy) _dialogue_tree _current_state))
  (bind (_greetings _choice _overlay) (Utilities|Struct|BreakTree_Struct _item))
  (bind _overlay_replies (Utilities|Struct|BreakOverlay_Struct _overlay))
  (bind _greetings_replies (Utilities|Struct|BreakGreetings_Struct _greetings))
  ;[1 1 1] checks validness of greet and choice in dialogue struct, for closing dialogue in unfinished situation(choice leads to uncreated tree)
  ; (if choice or state doesn't exist, skip /or finish dialogue to prevent jamming on it)
  (switch int Type?
    (:Default
      _)
    (:0
      _)
    (:1
      (if (Utilities|Array|IsValidIndex _choice) ; checks if at least one choice exist and not empty, and at the same time checks if greet doesn't exits the current dialogue(if so set choice to unexisting)
        ;;[1 1 1] valid choice
        (return false (Utilities|Enum|NotEqual(Enum) (.Choice_Text (Utilities|Struct|BreakChoice_Struct (Utilities|Array|Get(acopy) _choice))) (Utilities|Text|MakeLiteralText "")) false)
        (else
          (return false false false))))
    (:2
      (if (Utilities|Array|IsValidIndex _overlay_replies)
        ;;[1 1 1] valid overlay
        (return false false (Utilities|Enum|NotEqual(Enum) (Utilities|Array|Get(acopy) _overlay_replies) (Utilities|Text|MakeLiteralText "")))
        (else
          (return false false false)))))
  (if (Utilities|Array|IsValidIndex _greetings_replies) ; checks if at least one greet is valid from struct and not empty then set it as existing
    ;;[1 1 1] valid greet
    (return (Utilities|Enum|NotEqual(Enum) (Utilities|Array|Get(acopy) _greetings_replies) (Utilities|Text|MakeLiteralText "")) false false)
    (else
      (return false false false))))

(fn CastCharacterAnimSound
  (params (Sound? :type Boolean) (Anim_Montage :type Anim%20Montage%20Object%20Reference) (Current_Cue :type Sound%20Cue%20Object%20Reference) (CharIndex :type Integer))
  ;[1 1 1] reference func to easy change cast to needed Character class that plays anim or sound
  ; this is used in Dialogue_HUD and BP_Overlay_Text (this cast need only for playing animation and sound, and works only with character blueprint)
  ; so basicly it makes dynamic cast by pre-made classes list from enum_CharacterClasses so you wont need to find every cast for each character and change it manually
  ; you just add additional casts to your own classes of npc characters
  (LocalVariables|SetCurrentAnim Anim_Montage)
  (LocalVariables|SetCurrentCue Current_Cue)
  (bind (_actor_ _class_) (Casts|CalculateCast CharIndex))
  ;;[0.1686 0.4752 1] pure cast to box and mannequin character
  ;; (add more characters if you need)
  ;; (right click and convert default cast to pure)
  (LocalVariables|SetCurrentActor _actor_)
  (if (or (.bSuccess (Utilities|Casting|CastToBP_ThirdPersonCharacter _actor_)) (.bSuccess (Utilities|Casting|CastToBP_BoxCharacter _actor_)))
    (if Sound? ; this event fires by sequence, separately for anim and sound
      (bind _returnvalue (Audio|SpawnSoundAttached (LocalVariables|GetCurrentCue) (Variables|/Script/Engine.Character|GetMesh (Utilities|Select :Index _class_ :NewEnumerator0 (.AsBP%20Third%20Person%20Character (Utilities|Casting|CastToBP_ThirdPersonCharacter _actor_)) :NewEnumerator1 (.AsBP%20Box%20Character (Utilities|Casting|CastToBP_BoxCharacter _actor_)))) "None" "0, 0, 0" "0, 0, 0" "KeepRelativeOffset" true)) ; spawn sound(you can edit variables)
      (return _returnvalue) ; returns the current sound for stopping it inside widgets
      (else
        (Animation|PlayAnimMontage (Utilities|Select :Index _class_ :NewEnumerator0 (.AsBP%20Third%20Person%20Character (Utilities|Casting|CastToBP_ThirdPersonCharacter _actor_)) :NewEnumerator1 (.AsBP%20Box%20Character (Utilities|Casting|CastToBP_BoxCharacter _actor_))) (LocalVariables|GetCurrentAnim) 1.0 "None") ; play anim montage for dialogue
      ))
    (else
      ;;[1 1 1] print string on anim fail cast
      (Development|PrintString "Set Character Anim is Failed!")
      ;[1 1 1] play sound if target is not character class, sound will be attached to root component
      (if Sound?
        (bind _returnvalue_2 (Audio|SpawnSoundAttached (LocalVariables|GetCurrentCue) (VehicleSound|GetRootComponent (LocalVariables|GetCurrentActor)) "None" "0, 0, 0" "0, 0, 0" "KeepRelativeOffset" true)) ; spawn sound(you can edit variables)
        (return _returnvalue_2) ; returns the current sound for stopping it inside widgets
        (else
          _))))
  (return 0) ; Return no sound
)

(fn ShowOverlayName
  (bind _returnvalue (Game|GetPlayerCharacter 0))
  (bind _returnvalue_2 (Components|GetOwner))
  (bind _dialogue_settings (Variables|Default|GetDialogue_Settings))
  (bind _hide_floating_overlay_ (Utilities|Struct|BreakDialogue_Settings_Struct _dialogue_settings))
  ;[1 1 1] shows the overlay name based on distance and turns this off if dialogue is started or distance is far
  (Utilities|IsValid (Variables|NonEditable|GetDialogue_Overlay) ; cannot start if dialogue overlay is active
    (:Is%20Valid
      (if _hide_floating_overlay_ ; check if we need to hide overlay, then show name
        (if (!= _returnvalue _returnvalue_2) :!label _label ; ignore self character
          (if (Variables|NonEditable|GetInDialogue?) ; if in dialogue destroy the overlay name if exist
            (if _hide_floating_overlay_ ; show name even in dialogue, because overlay is hidden
              (if (< (Transformation|GetDistanceTo _returnvalue _returnvalue_2) 128.0) :!label _label_2
                (Utilities|IsValid (Variables|NonEditable|GetName_Overlay) ; start if invalid
                  (:Is%20Not%20Valid
                    (bind _returnvalue_3 (Game|SpawnActorfromClass "/Game/Dialogue_Pack/Blueprints/Dialogue/BP_Overlay_Text.BP_Overlay_Text_C" (Transformation|GetActorTransform (Components|GetOwner)) "AlwaysSpawn" 0 0))
                    (bind _output_get (Variables|NonEditable|SetName_Overlay _returnvalue_3))
                    (Default|StartOverlay _output_get self (Variables|NonEditable|GetDialogue_HUD) true false)))
                (else
                  (Utilities|IsValid (Variables|NonEditable|GetName_Overlay) :!label _label_3 ; destroy if valid
                    (:Is%20Valid
                      (Actor|DestroyActor (Variables|NonEditable|GetName_Overlay))))))
              (else
                (goto _label_3)))
            (else
              (goto _label_2))))
        (else
          (goto _label_3))))
    (:Is%20Not%20Valid
      (goto _label))))

(fn ShowOverlayDialogue
  (params (Unpaused? :type Boolean))
  ;[1 1 1] starts overlay sequence(non active dialogue, when npc just shows text above head while interacting,still can play anims and sound.
  ; consider overlay name and overlay dialogue shares the same blueprint
  ; (so if dialogue will be started the name will be destroyed until overlay dialogue was end)
  (Utilities|IsValid (Variables|NonEditable|GetDialogue_Overlay) ; interacting can be done if old sequence was finished
    (:Is%20Not%20Valid
      (bind _returnvalue (Game|SpawnActorfromClass "/Game/Dialogue_Pack/Blueprints/Dialogue/BP_Overlay_Text.BP_Overlay_Text_C" (Transformation|GetActorTransform (Components|GetOwner)) "AlwaysSpawn" 0 0))
      (bind _output_get (Variables|NonEditable|SetDialogue_Overlay _returnvalue))
      (Default|StartOverlay _output_get self (Variables|NonEditable|GetDialogue_HUD) false Unpaused?))))

(fn SetActors
  ;[1 1 1] sets the base dialogue actor and player character into last indexes of array
  ; (last is player, penultimate is base npc)
  (Variables|NonEditable|SetCharacters_List (.Characters_List (Utilities|Struct|BreakNPC_Additional_Settings_Struct (Variables|Default|GetCharacters_Settings))))
  (Utilities|Array|SetArrayElem (Variables|NonEditable|GetCharacters_List) (+ (Utilities|Array|LastIndex (Variables|NonEditable|GetCharacters_List)) 1) (Components|GetOwner) true)
  (Utilities|Array|SetArrayElem (Variables|NonEditable|GetCharacters_List) (+ (Utilities|Array|LastIndex (Variables|NonEditable|GetCharacters_List)) 1) (Game|GetPlayerCharacter 0) true))

(fn CalculateCast
  (params (CharacterIndex :type Integer))
  (bind _characters_list (Variables|NonEditable|GetCharacters_List))
  ;[1 1 1] calculate character's cast actor(npc or player) - which exactly npc from current reply, and their class from enum by index
  (return (Utilities|Array|Get(acopy) (Variables|NonEditable|GetCharacters_List) CharacterIndex) (select (== (Utilities|Array|LastIndex _characters_list) CharacterIndex) (.Player_Class (Utilities|Struct|BreakPlayer_Settings_Struct (Variables|Default|GetPlayer_Settings))) (select (== (- (Utilities|Array|LastIndex _characters_list) 1) CharacterIndex) (.NPC_Class (Utilities|Struct|BreakNPC_Settings_Struct (Variables|Default|GetNPC_Settings))) (Utilities|Array|Get(acopy) (.Characters_Class (Utilities|Struct|BreakNPC_Additional_Settings_Struct (Variables|Default|GetCharacters_Settings))) CharacterIndex)))))

(fn SpawnWidget
  (params (Overlays? :type Boolean))
  ;[1 1 1] spawn main dialogue widget, and store dialogue component inside(if overlays is true then make widget hidden)
  (bind _returnvalue (UserInterface|CreateWidget "/Game/Dialogue_Pack/Blueprints/Dialogue/HUD/Dialogue_HUD.Dialogue_HUD_C"))
  (bind _output_get (Variables|NonEditable|SetDialogue_HUD _returnvalue))
  (Variables|/Game/Dialogue_Pack/Blueprints/Dialogue/HUD/Dialogue_HUD.Dialogue_HUD_C|SetDialogueComponent _output_get self)
  (UserInterface|Viewport|AddtoViewport (Variables|NonEditable|GetDialogue_HUD) -1) ; order is -1 for not being top of focus(if you have other widgets)
  (if Overlays?
    (Default|HideWidgets (Variables|NonEditable|GetDialogue_HUD))))

(fn PauseOverlay
  (bind _returnvalue (Game|GetPlayerCharacter 0))
  (bind _returnvalue_2 (Components|GetOwner))
  (bind _returnvalue_3 (Components|GetOwner))
  (bind _dialogue_overlay (Variables|NonEditable|GetDialogue_Overlay))
  ;[1 1 1] pause the overlay dialogue, when actor pass the distance (also call dispatcher event for level blueprint)
  (if (!= _returnvalue _returnvalue_2) ; ignore self character
    (if (> (Transformation|GetDistanceTo _returnvalue _returnvalue_2) 5e+02)
      (if (not (Variables|NonEditable|GetPaused?))
        (Utilities|IsValid _dialogue_overlay
          (:Is%20Valid
            (Default|EndPaused _dialogue_overlay)
            (Default|CallDispPaused _returnvalue_3 true) ; calls dispatcher for events for needs(like to stop character's movement when dialogue is out of range)
            (Variables|NonEditable|SetPaused? true))))
      (elif (Variables|NonEditable|GetPaused?)
        (bind _active_dialogue_ (UpdateState|CheckDialogue))
        (if (not _active_dialogue_)
          (CallFunction|StartDialogue)
          (Default|CallDispPaused _returnvalue_3 false)
          (Variables|NonEditable|SetPaused? false))))))

(fn CheckDialogue
  ;[1 1 1] check active dialogue by getting all widgets of class(and check their stored dialogue component's In Dialogue Bool)
  ; if any 1 is valid, then dialogue cannot be started, if there is no active dialogues then it will start
  (bind _foundwidgets (Widget|GetAllWidgetsOfClass "/Game/Dialogue_Pack/Blueprints/Dialogue/HUD/Dialogue_HUD.Dialogue_HUD_C" false)) ; get all widgets of class Dialogue_HUD
  (bind _array_element (Utilities|Array|ForEachLoopwithBreak _foundwidgets :!label _label) ; strafe through every loop of widget
    (:LoopBody
      (Utilities|IsValid _array_element ; check if there is already valid widgets
        (:Is%20Valid
          (Utilities|IsValid (Variables|/Game/Dialogue_Pack/Blueprints/Dialogue/HUD/Dialogue_HUD.Dialogue_HUD_C|GetDialogueComponent _array_element) ; check if character was not destroyed
            (:Is%20Valid
              (if (Variables|BP_Dialogue_Component_C|GetInDialogue? (Variables|/Game/Dialogue_Pack/Blueprints/Dialogue/HUD/Dialogue_HUD.Dialogue_HUD_C|GetDialogueComponent _array_element))
                (Utilities|FlowControl|Sequence ; if there is at least one active dialogue break loop and set bool
                  (:then_0
                    (goto _label Break))
                  (:then_1
                    (return true)))))))))
    (:Completed
      (return false) ; if there was no active dialogues then set bool false at end
    )))

(fn SweepPlayer
  (params (bSweep :type Boolean) (Distance? :type Float%20%28single-precision%29))
  (bind _returnvalue (Components|GetOwner))
  (bind _returnvalue_2 (Game|GetPlayerCharacter 0))
  ;[1 1 1] stop velocity. and sweep player, to fix the distance.(warning, if player is on edge of map he can fall down)
  ; distance between player and npc will be 150 units(equal to capsules at dialogue cams BP)
  (Variables|/Script/Engine.MovementComponent|SetVelocity (Variables|/Script/Engine.Character|GetCharacterMovement _returnvalue_2) "0, 0, 0")
  (Transformation|SetActorLocation _returnvalue_2 (+ (* (Transformation|GetActorForwardVector _returnvalue) Distance?) (Transformation|GetActorLocation _returnvalue)) bSweep false))

(fn SweepNPC
  (params (bSweep :type Boolean) (Distance :type Float%20%28single-precision%29))
  (bind _returnvalue (Components|GetOwner))
  (bind _returnvalue_2 (Game|GetPlayerCharacter 0))
  (bind _returnvalue_3 (Actor|GetComponentbyClass _returnvalue "/Script/Engine.CharacterMovementComponent"))
  ;[1 1 1] sweep npc to fix location
  (Utilities|IsValid _returnvalue_3 ; get if actor have character movement
    (:Is%20Valid
      (Variables|/Script/Engine.MovementComponent|SetVelocity _returnvalue_3 "0, 0, 0") ; if character set velocity to 0
    )
    (:Is%20Not%20Valid
      _))
  (Transformation|SetActorLocation _returnvalue (+ (* (Transformation|GetActorForwardVector _returnvalue_2) Distance) (Transformation|GetActorLocation _returnvalue_2)) bSweep false) ; fix npc's location
)

(fn RotateNPC
  (bind _returnvalue (Components|GetOwner))
  (bind _returnvalue_2 (Transformation|GetActorRotation _returnvalue))
  (bind (_roll _pitch) (Math|Rotator|BreakRotator _returnvalue_2))
  ;[1 1 1] rotate npc towards player
  (Transformation|SetActorRotation (Components|GetOwner) (Math|Rotator|MakeRotator _roll _pitch (.Yaw (Math|Rotator|BreakRotator (Math|Rotator|FindLookatRotation (Transformation|GetActorLocation (Components|GetOwner)) (Transformation|GetActorLocation (Game|GetPlayerCharacter 0))))))))

(fn RotatePlayer
  (bind _returnvalue (Game|GetPlayerCharacter 0))
  (bind _returnvalue_2 (Components|GetOwner))
  (bind _returnvalue_3 (Transformation|GetActorRotation _returnvalue))
  (bind (_roll _pitch) (Math|Rotator|BreakRotator _returnvalue_3))
  ;[1 1 1] rotate player towards NPC, and check if it was success
  (Transformation|SetActorRotation (Game|GetPlayerCharacter 0) (Math|Rotator|MakeRotator _roll _pitch (.Yaw (Math|Rotator|BreakRotator (Math|Rotator|FindLookatRotation (Transformation|GetActorLocation (Game|GetPlayerCharacter 0)) (Transformation|GetActorLocation _returnvalue_2))))))
  (return (Math|Float|NearlyEqual(Float) (.Yaw (Math|Rotator|BreakRotator (Math|Rotator|Delta(Rotator) _returnvalue_3 (Transformation|GetActorRotation _returnvalue_2)))) 0.0 1e+01)))