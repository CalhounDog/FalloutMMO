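; BP_NPC_Updater changes an NPC's dialogue setup once, triggered by a quest event or dialogue choice.
; On BeginPlay it binds to BP_Quest_Actor's create/update dispatchers and the choice NPC's BP_Dialogue_Component, filtering by quest name, progress, completion or dialogue state and selection.
; The first match optionally sets the target's state, name and deactivation (sentinel defaults skip changes) and destroys listed actors.
; It then fires the quest actor's dispatcher with its settings for the Level Blueprint.
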(event Custom|QuestCreate
  (params (QuestName :type Name))
  ;[0.2135 1 0.8498] gets QuestName if equal to created quest name
  (if (Utilities|Name|Equal(Name) QuestName (Variables|Quest_Condition|GetQuest_Name))
    ;[0.2135 1 0.8498] get active bool
    (if (Variables|Quest_Condition|GetQ_CreateEvent?)
      ;[0.2135 1 0.8498] update values, consider if value was unchanged nothing will happen
      (CallFunction|UpdateEvents (Variables|Result|GetNPC_Update)) ; Update NPC variables
    )))

(event Custom|QuestUpdate
  (params (QuestName :type Name) (Finished? :type Boolean) (CurrentProgress :type Integer))
  ;[0.5378 0.235 1] compare QuestName to updated one, and compare finished by complete bool
  (if (Utilities|Name|Equal(Name) QuestName (Variables|Quest_Condition|GetQuest_Name))
    (if (and Finished? (Variables|Quest_Condition|GetQ_CompleteEvent?))
      ;[0.5378 0.235 1] update variables(on quest completed or updated)
      (CallFunction|UpdateEvents (Variables|Result|GetNPC_Update) :!label _label) ; Update NPC variables
      (else
        ;[0.5378 0.235 1] on updated bool
        (if (Variables|Quest_Condition|GetQ_UpdateEvent?)
          (if (== CurrentProgress (Variables|Quest_Condition|GetQ_UpdateAtProgress?))
            (goto _label)))))))

(event Custom|ChoiceEvent
  (bind _d_choiceatselection_ (Variables|ChoiceCondition|GetD_ChoiceAtSelection?))
  (bind _npc_choice (Variables|ChoiceCondition|GetNPC_Choice))
  (bind _returnvalue (Actor|GetComponentbyClass _npc_choice "/Game/Dialogue_Pack/Blueprints/Dialogue/BP_Dialogue_Component.BP_Dialogue_Component_C"))
  ;[0.3102 0.5602 1] NPC Choice Event
  (if (Variables|ChoiceCondition|GetD_ChoiceEvent?) ; get if choice bool
    (if (== (Variables|/Game/Dialogue_Pack/Blueprints/Dialogue/BP_Dialogue_Component.BP_Dialogue_Component_C|GetCurrent_State _returnvalue) (Variables|ChoiceCondition|GetD_EventState?)) ; if current state of dialogue equals to event state
      (if (== _d_choiceatselection_ -1) ; if selection index of choice to given(if -1 skip this)
        (CallFunction|UpdateEvents (Variables|Result|GetNPC_Update) :!label _label) ; update events
        (elif (== (Variables|/Game/Dialogue_Pack/Blueprints/Dialogue/BP_Dialogue_Component.BP_Dialogue_Component_C|GetChosen_Index _returnvalue) _d_choiceatselection_)
          (goto _label))))))

(event Custom|UpdateEvents
  (params (NPC_Reference :type Actor%20Object%20Reference))
  ;[1 0.4134 0] this "Event" sets every func by NPC reference,
  ; updates each changed variable on certain event
  (if (not (Variables|Components|GetDone?)) ; does once, to prevent bugs
    (Variables|Components|SetDone? true)
    (CallFunction|UpdateState NPC_Reference) ; update NPC's state
    (CallFunction|UpdateName NPC_Reference) ; update NPC's name
    (CallFunction|UpdateActive? NPC_Reference) ; update NPC's active state
    (CallFunction|DestroyActors?) ; destroy given actors
    (Default|CallDispLevel (Variables|Components|GetBP_Quest_Actor) (Variables|Result|GetNPC_Update) (Utilities|Struct|MakeUpdater_Struct (Variables|Quest_Condition|GetQuest_Name) (Variables|Quest_Condition|GetQ_CreateEvent?) (Variables|Quest_Condition|GetQ_UpdateEvent?) (Variables|Quest_Condition|GetQ_UpdateAtProgress?) (Variables|Quest_Condition|GetQ_CompleteEvent?) (Variables|ChoiceCondition|GetNPC_Choice) (Variables|ChoiceCondition|GetD_ChoiceEvent?) (Variables|ChoiceCondition|GetD_EventState?) (Variables|ChoiceCondition|GetD_ChoiceAtSelection?))) ; calls dispatcher event within quest actor, for level blueprint to access event\nIt stores every necessary value to struct and fires dispatcher event
  ))

(event EventBeginPlay
  (bind _npc_choice (Variables|ChoiceCondition|GetNPC_Choice))
  (bind _returnvalue (Actor|GetComponentbyClass _npc_choice "/Game/Dialogue_Pack/Blueprints/Dialogue/BP_Dialogue_Component.BP_Dialogue_Component_C"))
  ;[0.1655 0.6617 1] gets reference of quest actor
  (bind _outactors (Actor|GetAllActorsOfClass "/Game/Dialogue_Pack/Blueprints/Quest/BP_Quest_Actor.BP_Quest_Actor_C"))
  (Utilities|IsValid (Utilities|Array|Get(acopy) _outactors)
    (:Is%20Valid
      (Variables|Components|SetBP_Quest_Actor (Utilities|Array|Get(acopy) _outactors))
      ;[1 0.1904 0.1107] get dispatcher events, they fire when quest creates, updates or finishes.
      (EventDispatchers|BindEventtoDispCreate (Variables|Components|GetBP_Quest_Actor) (delegate Custom|QuestCreate))
      (EventDispatchers|BindEventtoDispUpdate (Variables|Components|GetBP_Quest_Actor) (delegate Custom|QuestUpdate))
      ;[0.3102 0.5602 1] NPC Choice Event
      (Utilities|IsValid _npc_choice ; checks if choice npc is valid
        (:Is%20Valid
          (Utilities|IsValid _returnvalue ; checks if it have dialogue component
            (:Is%20Valid
              (EventDispatchers|AssignDispChoice _returnvalue (delegate Custom|ChoiceEvent)) ; binds choice event
            )))))))

(fn ConstructionScript)

(fn UpdateState
  (params (NPC_Reference :type Actor%20Object%20Reference))
  (bind _returnvalue (Actor|GetComponentbyClass NPC_Reference "/Game/Dialogue_Pack/Blueprints/Dialogue/BP_Dialogue_Component.BP_Dialogue_Component_C"))
  (bind _set_currentstate (Variables|Result|GetSet_CurrentState))
  ;[1 1 1] this changes state, consider if value is -1(default) nothing will happen
  (Utilities|IsValid NPC_Reference
    (:Is%20Valid
      (if (!= _set_currentstate -1)
        (Variables|/Game/Dialogue_Pack/Blueprints/Dialogue/BP_Dialogue_Component.BP_Dialogue_Component_C|SetCurrent_State _returnvalue _set_currentstate)
        (Default|UpdateQuestions _returnvalue) ; update questions at state change
      ))
    (:Is%20Not%20Valid
      _))
  (return))

(fn UpdateName
  (params (NPC_Reference :type Actor%20Object%20Reference))
  (bind _set_name (Variables|Result|GetSet_Name))
  ;[1 1 1] updates name on given event, consider that if name is empty nothing will happen
  (Utilities|IsValid NPC_Reference
    (:Is%20Valid
      (if (Utilities|Enum|NotEqual(Enum) _set_name "")
        (Variables|/Game/Dialogue_Pack/Blueprints/Dialogue/BP_Dialogue_Component.BP_Dialogue_Component_C|SetOwnerName (Actor|GetComponentbyClass NPC_Reference "/Game/Dialogue_Pack/Blueprints/Dialogue/BP_Dialogue_Component.BP_Dialogue_Component_C") _set_name)))
    (:Is%20Not%20Valid
      _))
  (return))

(fn DestroyActors?
  ;[1 1 1] destroy the given array of actors, if any actor from array is in current dialogue(it will stop dialogue before destroying)
  (for _array_element (Variables|Result|GetDestroyActors?)
    (Actor|DestroyActor _array_element))
  (return))

(fn UpdateActive?
  (params (NPC_Reference :type Actor%20Object%20Reference))
  (bind _set_deactivate (Variables|Result|GetSet_Deactivate))
  ;[1 1 1] this sets deactive value during event, if value is same nothing will happen
  (Utilities|IsValid NPC_Reference
    (:Is%20Valid
      (if (!= _set_deactivate -1) ; if value was unchanged nothing will happen
        (Variables|/Game/Dialogue_Pack/Blueprints/Dialogue/BP_Dialogue_Component.BP_Dialogue_Component_C|SetDeactive? (Actor|GetComponentbyClass NPC_Reference "/Game/Dialogue_Pack/Blueprints/Dialogue/BP_Dialogue_Component.BP_Dialogue_Component_C") (Utilities|Select :Index _set_deactivate :Option%200 false :Option%201 true))))
    (:Is%20Not%20Valid
      _))
  (return))